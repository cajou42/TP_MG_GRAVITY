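; BP_MG_Player is a player pawn with hand-written movement and jumping driven by Enhanced Input, without using physics.
; GravityMove applies swept world offsets by gravity Direction: actor rotation axes for Plane, control rotation projected onto the PlanetAttraction plane for Sphere.
; Tick integrates JumpVelocity and Gravity along world Z only, and a blocking hit resets the jump and sets IsGrounded.
; The line-trace ground check is disconnected, so nothing here clears IsGrounded.
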(event `self.ReceiveBeginPlay`
  (bind _asplayer_controller (cast `PlayerController` (`self.GetController`)))
  (`EnhancedInputSubsystemInterface.AddMappingContext` (pcsubsystem `EnhancedInputLocalPlayerSubsystem` _asplayer_controller) "/Game/Input/IMC_Player.IMC_Player" 0 (struct)))

(event `EnhancedInput|/Game/Input/IA_Move`
  (params (ActionValue :type "Vector Structure") (ElapsedSeconds :type "Float (double-precision)") (TriggeredSeconds :type "Float (double-precision)") (InputAction :type "InputAction Object Reference" :default "/Game/Input/IA_Move.IA_Move"))
  (:`Triggered`
    (set `self.XValue` ActionValue_X)
    (set `self.YValue` ActionValue_Y)
    (`self.GravityMove`)))

(event `EnhancedInput|/Game/Input/IA_Jump`
  (params (ActionValue :type Boolean) (ElapsedSeconds :type "Float (double-precision)") (TriggeredSeconds :type "Float (double-precision)") (InputAction :type "InputAction Object Reference" :default "/Game/Input/IA_Jump.IA_Jump"))
  (:`Started`
    (if (not (`self.hasJumped`))
      (set `self.hasJumped` true)
      (set `self.JumpVelocity` (`self.JumpForce`)))))

(event `self.ReceiveTick`
  (params (DeltaSeconds :type "Float (single-precision)"))
  (if (`self.IsGrounded`)
    (if (`self.hasJumped`)
      (`self.K2_AddActorWorldOffset` (`KismetMathLibrary.MakeVector` 0.0 0.0 (* (`self.JumpVelocity`) (`GameplayStatics.GetWorldDeltaSeconds`))) true)
      (`self.IsFalling`))
    (else
      (`self.IsFalling`))))

(event `IsFalling`
  (bind _output_get (set `self.JumpVelocity` (- (`self.JumpVelocity`) (* (`self.Gravity`) (`GameplayStatics.GetWorldDeltaSeconds`)))))
  (bind _sweephitresult (`self.K2_AddActorWorldOffset` (`KismetMathLibrary.MakeVector` 0.0 0.0 (* _output_get (`GameplayStatics.GetWorldDeltaSeconds`))) true))
  (if (`GameplayStatics.BreakHitResult` _sweephitresult)
    (set `self.hasJumped` false)
    (set `self.IsGrounded` true)
    (set `self.JumpVelocity` 0.0)))

(fn `GravityMove`
  (bind _returnvalue (`self.GetControlRotation`))
  (bind _speed (`self.speed`))
  (bind _planetattraction (`self.PlanetAttraction`))
  (bind _speed_2 (`self.speed`))
  (bind _returnvalue_x (`KismetMathLibrary.BreakVector` (`KismetMathLibrary.ProjectVectorOnToPlane` (`KismetMathLibrary.GetForwardVector` _returnvalue) _planetattraction)))
  (bind _returnvalue_2 (`KismetMathLibrary.Conv_TransformToMatrix` (`KismetMathLibrary.MakeTransform` (0.0 0.0 0.0) (`self.K2_GetActorRotation`))))
  (bind (_returnvalue_x_2 _returnvalue_y) (`KismetMathLibrary.BreakVector` (`KismetMathLibrary.ProjectVectorOnToPlane` (`KismetMathLibrary.GetRightVector` _returnvalue) _planetattraction)))
  (bind _returnvalue_x_3 (`KismetMathLibrary.BreakVector` (`KismetMathLibrary.Matrix_GetScaledAxis` _returnvalue_2 "X")))
  (bind (_returnvalue_x_4 _returnvalue_y_2) (`KismetMathLibrary.BreakVector` (`KismetMathLibrary.Matrix_GetScaledAxis` _returnvalue_2 "Y")))
  (switch `GravityDirection` (`self.Direction`)
    (:`GD_Plane`
      (`self.K2_AddActorWorldOffset` (`KismetMathLibrary.MakeVector` (* (`self.YValue`) _speed _returnvalue_y_2) (* (`self.XValue`) _speed _returnvalue_x_3)) true))
    (:`GD_Sphere`
      (`self.K2_AddActorWorldOffset` (`KismetMathLibrary.MakeVector` (* (`self.XValue`) _returnvalue_x _speed_2) (* _speed_2 _returnvalue_y (`self.YValue`))) true))))

(fn `UserConstructionScript`)